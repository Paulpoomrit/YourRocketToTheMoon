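; BP_UrBunny_Child is a bunny character child Blueprint that shows a thinking emote bubble when the bear character is near.
; Overlap with a BP_BearCharacter or its subclass runs after the parent's begin-overlap logic and makes BubbleEmotesThinking visible.
; When that overlap ends, the bubble hides after a one-second delay, without checking whether the bear has re-entered.
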(event EventBeginPlay
  (|CallParentFunction) ; This node is disabled and will not be called.\nDrag off pins to build functionality.
)

(event Collision|EventActorBeginOverlap
  (params (OtherActor :type Actor%20Object%20Reference))
  (|CallParentFunction OtherActor)
  (if (Utilities|ClassIsChildOf (Utilities|GetClass OtherActor) "/Game/2_Blueprints/1_BearCharacter/BP_BearCharacter.BP_BearCharacter_C")
    (Rendering|SetVisibility (Variables|Default|Getbubble_emotes_thinking) true false)))

(event EventTick
  (params (DeltaSeconds :type Float%20%28single-precision%29))
  (|CallParentFunction DeltaSeconds) ; This node is disabled and will not be called.\nDrag off pins to build functionality.
)

(event Collision|EventActorEndOverlap
  (params (OtherActor :type Actor%20Object%20Reference))
  (if (Utilities|ClassIsChildOf (Utilities|GetClass OtherActor) "/Game/2_Blueprints/1_BearCharacter/BP_BearCharacter.BP_BearCharacter_C")
    (Utilities|FlowControl|Delay 1.0)
    (Rendering|SetVisibility (Variables|Default|Getbubble_emotes_thinking) false false)))

(fn ConstructionScript
  (|CallParentFunction))