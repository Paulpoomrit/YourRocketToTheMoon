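; A variant of the UrBunny character for the Void level that stays dormant during the Void intro.
; On BeginPlay it copies the intro flag from BP_GameInstance, then either hides itself with tick and collision disabled, or runs parent startup and restores all three.
; The same cached flag gates the parent's overlap and tick logic, so inherited behavior runs only outside the intro.
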(event EventBeginPlay
  (bind _asbp_game_instance (Utilities|Casting|CastToBP_GameInstance (Game|GetGameInstance)))
  (bind _output_get (Variables|Default|SetIs%20in%20the%20Void%20Intro (Variables|/Game/0_Levels/BP_GameInstance.BP_GameInstance_C|GetisInTheVoidIntro _asbp_game_instance)))
  (if _output_get
    (Development|PrintString "in the void!")
    ;[0.4762 0.3021 0.8994] hide!
    (Rendering|SetActorHiddenInGame true)
    (Actor|Tick|SetActorTickEnabled false)
    (Collision|SetActorEnableCollision false)
    (else
      (|CallParentFunction)
      ;[0.4762 0.3021 0.8994] un-hide!
      (Rendering|SetActorHiddenInGame false)
      (Actor|Tick|SetActorTickEnabled true)
      (Collision|SetActorEnableCollision true))))

(event Collision|EventActorBeginOverlap
  (params (OtherActor :type Actor%20Object%20Reference))
  (if (Variables|Default|GetIs%20in%20the%20Void%20Intro)
    (Development|PrintString "in the void!")
    (else
      (|CallParentFunction OtherActor))))

(event EventTick
  (params (DeltaSeconds :type Float%20%28single-precision%29))
  (if (not (Variables|Default|GetIs%20in%20the%20Void%20Intro))
    (|CallParentFunction DeltaSeconds)))

(fn ConstructionScript
  (|CallParentFunction))