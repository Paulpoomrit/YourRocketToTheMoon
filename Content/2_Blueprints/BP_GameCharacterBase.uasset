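; Base Blueprint for game characters that can be interacted with to show dialogue through the game mode's HUD widget.
; Interact notifies the instigator, sets an interaction lock and shows the current DT_Dialogue row, while FinishInteraction clears the lock.
; Each row stores the next row's name, so ShowNextLine walks the chain and returns false when it ends, resetting the current row to None.
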(event EventBeginPlay
  (Rendering|SetCastShadow (Variables|Default|GetDialogueIndicator) false)
  (bind _asgm_your_rocket_to_the_moon (Utilities|Casting|CastToGM_YourRocketToTheMoon (Game|GetGameMode)))
  (Variables|Default|SetGameMode _asgm_your_rocket_to_the_moon))

(event Collision|EventActorBeginOverlap
  (params (OtherActor :type Actor%20Object%20Reference)))

(event EventTick
  (params (DeltaSeconds :type Float%20%28single-precision%29)))

(event EventInteract
  (params (Instigator :type BP%20Game%20Character%20Base%20Object%20Reference))
  (CallFunction|StartInteraction Instigator)
  (CallFunction|StartInteraction)
  (CallFunction|ShowDialogueLine))

(event EventFinishInteraction
  (CallFunction|EndInteraction))

(fn ConstructionScript)

(fn ShowDialogueLine
  (bind _returnvalue (Utilities|GetDataTableRow "/Game/4_DataTables/DT_Dialogue.DT_Dialogue" (Variables|Default|GetCurrentRowName))
    (:then
      (Default|ShowDialogue (Variables|/Game/2_Blueprints/0_ProjectSettings/GM_YourRocketToTheMoon.GM_YourRocketToTheMoon_C|GetHUDWidget (Variables|Default|GetGameMode)) (.DialogueText (Utilities|Struct|BreakS_DialogueData _returnvalue)))
      (Variables|Default|SetNextRow (.NextRow (Utilities|Struct|BreakS_DialogueData _returnvalue)))
      (return))))

(fn StartInteraction
  (Variables|Default|SetIsInteractingLocked true))

(fn EndInteraction
  (Variables|Default|SetIsInteractingLocked false))

(fn ShowNextLine
  (if (Utilities|Array|IsEmpty (Variables|Default|GetNextRow))
    (Variables|Default|SetCurrentRowName "None")
    (return false)
    (else
      (Variables|Default|SetCurrentRowName (Utilities|String|StringToName (Variables|Default|GetNextRow)))
      (CallFunction|ShowDialogueLine)
      (return true))))