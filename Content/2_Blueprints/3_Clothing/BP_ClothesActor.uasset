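; BP_ClothesActor is a clickable clothing item that advances through stages on each click, tracked by a Count state.
; Early states nudge it along the Y axis with movement input.
; State 2 plays the ClothesOut level sequence once, pausing it after a short delay before setting state 3.
; A click in state 3 destroys the actor and calls CallNextClothes.
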(event EventBeginPlay)

(event Collision|EventActorBeginOverlap
  (params (OtherActor :type Actor%20Object%20Reference)))

(event EventTick
  (params (DeltaSeconds :type Float%20%28single-precision%29)))

(event MouseInput|EventActorOnClicked
  (params (ButtonPressed :type Key%20Structure :default "None"))
  (if (== (Variables|Default|GetCount) 0)
    (Pawn|Input|AddMovementInput "0.000000,1.000000,0.000000" 0.1 false)
    (Variables|Default|SetCount 2)
    (elif (== (Variables|Default|GetCount) 1)
      (Pawn|Input|AddMovementInput "0.000000,-1.000000,0.000000" 0.1 false)
      (Variables|Default|SetCount 0)
      (elif (== (Variables|Default|GetCount) 2)
        (Utilities|FlowControl|DoOnce false
          (:Completed
            (bind _returnvalue (Sequencer|Player|CreateLevelSequencePlayer "/Game/0_Levels/Sequencer/FoldingLevel/ClothesOut.ClothesOut"))
            (Sequencer|Player|Play _returnvalue :!class /Script/MovieScene.MovieSceneSequencePlayer)
            (Utilities|FlowControl|Delay 0.5)
            (Sequencer|Player|Pause _returnvalue)
            (Variables|Default|SetCount 3)))
        (elif (== (Variables|Default|GetCount) 3)
          (Actor|DestroyActor)
          (Default|CallNextClothes))))))

(fn ConstructionScript)