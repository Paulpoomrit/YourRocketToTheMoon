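; BP_Clothes is a clickable clothing actor that prints "fold!" on each click, apparently an early stub of a folding interaction.
; A Count variable steps through the clicks: the first adds a small movement input along +Y, the second along -Y.
; Once Count reaches 2, further clicks only print the message.
; BeginPlay and the construction script only call their parents, and Tick and overlap are disabled.
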(event EventBeginPlay
  (|CallParentFunction))

(event Collision|EventActorBeginOverlap
  (params (OtherActor :type Actor%20Object%20Reference))
  (|CallParentFunction OtherActor) ; This node is disabled and will not be called.\nDrag off pins to build functionality.
)

(event EventTick
  (params (DeltaSeconds :type Float%20%28single-precision%29))
  (|CallParentFunction DeltaSeconds) ; This node is disabled and will not be called.\nDrag off pins to build functionality.
)

(event MouseInput|EventActorOnClicked
  (params (ButtonPressed :type Key%20Structure :default "None"))
  (Development|PrintString "fold!")
  (if (== (Variables|Default|Get%20Count) 0)
    (Pawn|Input|AddMovementInput "0.000000,1.000000,0.000000" 0.1 false)
    (Variables|Default|Set%20Count 1)
    (elif (== (Variables|Default|Get%20Count) 1)
      (Pawn|Input|AddMovementInput "0.000000,-1.000000,0.000000" 0.1 false)
      (Variables|Default|Set%20Count 2)
      (elif (== (Variables|Default|Get%20Count) 2)
        _))))

(fn ConstructionScript
  (|CallParentFunction))