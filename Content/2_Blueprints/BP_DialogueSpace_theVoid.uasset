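; Dialogue trigger for the Void level that hides and disables itself during the Void intro, per a GameInstance flag.
; Overlapping it flags the final act on the GameInstance and calls for the final scene to unhide.
; Tick watches for the inherited dialogue row to become None, then once swaps the bear's Enhanced Input context to walk-away and fires a dispatcher.
; The walk-away prompt widget code is disconnected.
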(event Custom|walkAway
  (Development|PrintString "Hello")
  (bind _asbp_bear_void_2 (Utilities|Casting|CastToBP_Bear_Void2 (Game|GetPlayerCharacter 0)))
  (Input|RemoveMappingContext (PlayerController|LocalPlayerSubsystems|GetEnhancedInputLocalPlayerSubsystem (Game|GetPlayerController (Variables|/Script/Engine.Pawn|GetPlayerState _asbp_bear_void_2))) "/Game/2_Blueprints/0_BearPTT/Inputs/IMC_BearDefault.IMC_BearDefault" "(bIgnoreAllPressedKeysUntilRelease=True,bForceImmediately=False,bNotifyUserSettings=False)")
  (Input|AddMappingContext (PlayerController|LocalPlayerSubsystems|GetEnhancedInputLocalPlayerSubsystem (Game|GetPlayerController (Variables|/Script/Engine.Pawn|GetPlayerState _asbp_bear_void_2))) "/Game/2_Blueprints/0_BearPTT/Inputs/IMC_WalkAway.IMC_WalkAway" 0 "(bIgnoreAllPressedKeysUntilRelease=True,bForceImmediately=False,bNotifyUserSettings=False)")
  (Default|CallWalkAwayDispatcher))

(event EventBeginPlay
  (|CallParentFunction)
  (bind _asbp_game_instance (Utilities|Casting|CastToBP_GameInstance (Game|GetGameInstance)))
  (if (Variables|/Game/0_Levels/BP_GameInstance.BP_GameInstance_C|GetisInTheVoidIntro _asbp_game_instance)
    ;[0.4762 0.3021 0.8994] hide!
    (Rendering|SetActorHiddenInGame true)
    (Actor|Tick|SetActorTickEnabled false)
    (Collision|SetActorEnableCollision false)
    (else
      ;[0.4762 0.3021 0.8994] un-hide!
      (Rendering|SetActorHiddenInGame false)
      (Actor|Tick|SetActorTickEnabled true)
      (Collision|SetActorEnableCollision true))))

(event Collision|EventActorBeginOverlap
  (params (OtherActor :type Actor%20Object%20Reference))
  (|CallParentFunction OtherActor)
  (Variables|/Game/0_Levels/BP_GameInstance.BP_GameInstance_C|SetisInTheFinalAct (stale EventBeginPlay _asbp_game_instance) true)
  (Default|CallUnhideFinalScene))

(event EventTick
  (params (DeltaSeconds :type Float%20%28single-precision%29))
  (|CallParentFunction DeltaSeconds)
  (if (== (Variables|Default|GetCurrentRowName) "None")
    (Utilities|FlowControl|DoOnce false
      (:Completed
        (CallFunction|WalkAway)))))

(fn ConstructionScript
  (|CallParentFunction))