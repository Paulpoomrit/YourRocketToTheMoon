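; BP_PlayerBearPTT is the player pawn for BearPTT, limited to movement along the world X axis.
; On BeginPlay it adds the IMC_BearDefault Enhanced Input mapping context to its PlayerController.
; IA_Move feeds the X component of its input into AddMovementInput.
; Y-axis movement and an IsInteractingLocked check meant for blocking the character are present but unconnected, so neither runs.
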(event Input|EnhancedActionEvents|EnhancedInputActionIA_Move
  (params (ActionValue :type Vector%202D%20Structure) (ElapsedSeconds :type Float%20%28double-precision%29) (TriggeredSeconds :type Float%20%28double-precision%29) (InputAction :type Input%20Action%20Object%20Reference :default "/Game/2_Blueprints/0_BearPTT/Inputs/Actions/IA_Move.IA_Move"))
  (Pawn|Input|AddMovementInput "1.000000,0.000000,0.000000" (.x ActionValue) false))

(event EventBeginPlay
  (|CallParentFunction)
  (bind _asplayer_controller (Utilities|Casting|CastToPlayerController (Pawn|GetController)))
  (Input|AddMappingContext (PlayerController|LocalPlayerSubsystems|GetEnhancedInputLocalPlayerSubsystem _asplayer_controller) "/Game/2_Blueprints/0_BearPTT/Inputs/IMC_BearDefault.IMC_BearDefault" 0 "(bIgnoreAllPressedKeysUntilRelease=True,bForceImmediately=False,bNotifyUserSettings=False)"))

(event Collision|EventActorBeginOverlap
  (params (OtherActor :type Actor%20Object%20Reference))
  (|CallParentFunction OtherActor) ; This node is disabled and will not be called.\nDrag off pins to build functionality.
)

(event EventTick
  (params (DeltaSeconds :type Float%20%28single-precision%29))
  (|CallParentFunction DeltaSeconds) ; This node is disabled and will not be called.\nDrag off pins to build functionality.
)

(fn ConstructionScript
  (|CallParentFunction))