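; BP_NPC is an NPC Blueprint that chases the player when its IsRoaming flag is set.
; BeginPlay checks the flag and starts an AI MoveTo toward player pawn 0, which calls FollowPlayer again on success or failure, forming an endless follow loop.
; MoveRandomWithDelay, commented as free roaming, only runs a random retriggerable delay and is not called in this graph.
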(event Custom|MoveRandomWithDelay
  ;[0.4762 0.3021 0.8994] roam freely
  (Utilities|FlowControl|RetriggerableDelay (Math|Random|RandomFloatinRange 1.0 5.0)))

(event Custom|FollowPlayer
  (AI|AIMoveTo self "0, 0, 0" (Game|Player|GetPlayerPawn 0) 1e+02 false
    (:OnSuccess
      _)
    (:OnFail
      _))
  (CallFunction|FollowPlayer))

(event EventBeginPlay
  (|CallParentFunction)
  (if (Variables|Default|GetisRoaming)
    (AI|AIMoveTo self "0, 0, 0" (Game|Player|GetPlayerPawn 0) 1e+02 false
      (:OnSuccess
        _)
      (:OnFail
        _))
    (CallFunction|FollowPlayer)))

(fn ConstructionScript
  (|CallParentFunction))