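; Player bear character that triggers dialogue and cutscenes with the objects and characters it overlaps.
; Entering a dialogue space starts interaction with overlapping game characters, or queues that space if a dialogue is already running.
; The interact input advances speech-bubble lines in the HUD, then starts the next queued dialogue when one ends.
; Unplayed cutscenes notify on overlap and start on interact, only while the dialogue queue is empty.
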(event Input|EnhancedActionEvents|EnhancedInputActionIA_Interact
  (params (ActionValue :type Boolean) (ElapsedSeconds :type Float%20%28double-precision%29) (TriggeredSeconds :type Float%20%28double-precision%29) (InputAction :type Input%20Action%20Object%20Reference :default "/Game/2_Blueprints/0_BearPTT/Inputs/Actions/IA_Interact.IA_Interact"))
  (if (Variables|Default|GetIsInteractingLocked)
    (if (Default|FinishRevealing (Variables|/Game/3_UX_UI/WBP_HUD.WBP_HUD_C|GetWBP_SpeechBubble (Variables|/Game/2_Blueprints/0_ProjectSettings/GM_YourRocketToTheMoon.GM_YourRocketToTheMoon_C|GetHUDWidget (Variables|Default|GetGameMode))))
      (bind _lastinteractedobj (Variables|Default|GetlastInteractedObj)
        (:then
          ;[0.4762 0.3021 0.8994] Has next line?
          (bind _hasnextline (Class|BPIInteraction|ShowNextLine(Message) _lastinteractedobj))
          (if (not _hasnextline)
            ;[0.4762 0.3021 0.8994] End the dialogue interaction only if the revealing is complete && does not has next line
            (CallFunction|EndInteraction)
            (bind _asbp_game_character_base (Utilities|Casting|CastToBP_GameCharacterBase (Variables|Default|GetlastInteractedObj)))
            (Default|FinishInteraction _asbp_game_character_base)
            (Default|HideDialogue (Variables|/Game/3_UX_UI/WBP_HUD.WBP_HUD_C|GetWBP_SpeechBubble (Variables|/Game/2_Blueprints/0_ProjectSettings/GM_YourRocketToTheMoon.GM_YourRocketToTheMoon_C|GetHUDWidget (Variables|Default|GetGameMode))))
            ;[0.4762 0.3021 0.8994] If there's dialogue in queue
            (if (Utilities|Array|IsNotEmpty (Variables|Default|GetArrayOfDialogueSpace))
              (bind _output_get (Variables|Default|SetArray%20Element (Utilities|Array|Get(acopy) (Variables|Default|GetArrayOfDialogueSpace))))
              ;;[0.4762 0.3021 0.8994] If the obj/char has no dialogue option/ lines left -> skip interaction
              (Development|PrintString (Utilities|String|ToString(Name) (Variables|/Game/2_Blueprints/BP_GameCharacterBase.BP_GameCharacterBase_C|GetCurrentRowName _output_get)))
              (if (!= (Variables|/Game/2_Blueprints/BP_GameCharacterBase.BP_GameCharacterBase_C|GetCurrentRowName _output_get) "")
                (Default|Interact _output_get self)
                (Variables|Default|SetlastInteractedObj _output_get)
                (Utilities|Array|RemoveItem (Variables|Default|GetArrayOfDialogueSpace) _output_get)))))
        (:else)))
    (else
      (bind _array_element (Utilities|Array|ForEachLoopwithBreak (Collision|GetOverlappingActors (Variables|Default|GetInteractionCheck) "/Game/2_Blueprints/BP_Cutscene.BP_Cutscene_C" :!class /Script/Engine.PrimitiveComponent))
        (:LoopBody
          ;[0.4762 0.3021 0.8994] Enter cutscene if there's no dialogue left in the array
          (bind _asbp_cutscene (Utilities|Casting|CastToBP_Cutscene _array_element))
          (if (not (Variables|/Game/2_Blueprints/BP_DialogueSpace.BP_DialogueSpace_C|GetHasBeenInteractedWithOnce _asbp_cutscene))
            (if (== (Utilities|Array|Length (Variables|Default|GetArrayOfDialogueSpace)) 0)
              (Default|CallCutsceneEventDispatcher)
              (Variables|Default|SetinCutscene true))))))))

(event EventBeginPlay
  (|CallParentFunction))

(event Collision|EventActorBeginOverlap
  (params (OtherActor :type Actor%20Object%20Reference))
  (bind _returnvalue (Utilities|GetClass OtherActor))
  (|CallParentFunction OtherActor)
  (if (Utilities|ClassIsChildOf (Utilities|GetClass OtherActor) "/Game/2_Blueprints/BP_Cutscene.BP_Cutscene_C")
    ;[0.4762 0.3021 0.8994] Enter cutscene if there's no dialogue left in the array
    (bind _asbp_cutscene (Utilities|Casting|CastToBP_Cutscene OtherActor)
      (:then
        (if (not (Variables|/Game/2_Blueprints/BP_DialogueSpace.BP_DialogueSpace_C|GetHasBeenInteractedWithOnce _asbp_cutscene))
          (if (== (Utilities|Array|Length (Variables|Default|GetArrayOfDialogueSpace)) 0)
            (Default|CallCutsceneNotifier)
            (else
              ;[0.4762 0.3021 0.8994] Interacting with Dialogue Box
              (if (and (Utilities|ClassIsChildOf _returnvalue "/Game/2_Blueprints/BP_DialogueSpace.BP_DialogueSpace_C") (not (Utilities|ClassIsChildOf _returnvalue "/Game/2_Blueprints/BP_Cutscene.BP_Cutscene_C"))) :!label _label
                (bind _asbp_dialogue_space (Utilities|Casting|CastToBP_DialogueSpace OtherActor))
                (if (not (Variables|/Game/2_Blueprints/BP_DialogueSpace.BP_DialogueSpace_C|GetHasBeenInteractedWithOnce _asbp_dialogue_space))
                  (if (Variables|Default|GetIsInteractingLocked)
                    (Utilities|Array|Add (Variables|Default|GetArrayOfDialogueSpace) _asbp_dialogue_space)
                    (Variables|/Game/2_Blueprints/BP_DialogueSpace.BP_DialogueSpace_C|SetHasBeenInteractedWithOnce _asbp_dialogue_space true)
                    (Development|PrintString (Utilities|String|ToString(Name) (Variables|/Game/2_Blueprints/BP_GameCharacterBase.BP_GameCharacterBase_C|GetCurrentRowName _asbp_dialogue_space)))
                    (else
                      ;;[0.4762 0.3021 0.8994] If the player currently does not interact with any obj:
                      ;;;[0.4762 0.3021 0.8994] For each loop with break only let you interact with 1 obj at a time
                      (bind _array_element (Utilities|Array|ForEachLoopwithBreak (Collision|GetOverlappingActors (Variables|Default|GetInteractionCheck) 0 :!class /Script/Engine.PrimitiveComponent))
                        (:LoopBody
                          (if (!= _array_element self)
                            ;;;[0.4762 0.3021 0.8994] If the obj/char has no dialogue option/ lines left -> skip interaction
                            (bind _asbp_game_character_base (Utilities|Casting|CastToBP_GameCharacterBase _array_element))
                            (bind _output_get (Variables|Default|SetlastInteractedObj _array_element))
                            (bind _asbp_game_character_base_2 (Utilities|Casting|CastToBP_GameCharacterBase _output_get))
                            (if (!= (Variables|/Game/2_Blueprints/BP_GameCharacterBase.BP_GameCharacterBase_C|GetCurrentRowName _asbp_game_character_base_2) "")
                              (Rendering|SetVisibility (Variables|Default|Getbubble_emotes_thinking) false false)
                              (Default|Interact _asbp_game_character_base self)))))))))))
          (else
            (goto _label))))
      (:CastFailed
        (goto _label)))
    (else
      (goto _label))))

(event EventTick
  (params (DeltaSeconds :type Float%20%28single-precision%29))
  (|CallParentFunction DeltaSeconds) ; This node is disabled and will not be called.\nDrag off pins to build functionality.
)

(event Collision|EventActorEndOverlap
  (params (OtherActor :type Actor%20Object%20Reference))
  (bind _asbp_cutscene (Utilities|Casting|CastToBP_Cutscene OtherActor))
  (if (not (Variables|/Game/2_Blueprints/BP_DialogueSpace.BP_DialogueSpace_C|GetHasBeenInteractedWithOnce _asbp_cutscene))
    (Rendering|SetVisibility (Variables|/Game/2_Blueprints/BP_GameCharacterBase.BP_GameCharacterBase_C|Getbubble_emotes_thinking _asbp_cutscene) false false)))

(fn ConstructionScript
  (|CallParentFunction))

(fn ShowDialogueLine
  (|CallParentFunction))

(fn ShowNextLine
  (return false))

(fn CreateNewInstanceOfDialogueScene)